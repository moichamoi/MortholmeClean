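; BP_VitralPrincipal is the main stained-glass (vitral) actor, able to swap itself for an exploded version.
; When ToggleExplode fires with the ExplodeToggle flag set, it spawns BP_Exploded_VitralPrincipal at its transform, calls SetMaterial on that Geometry Collection and destroys itself.
; An unset flag or failed cast only prints a message.
; Indexed skin assignment to the intact mesh exists but is disconnected, and BeginPlay is empty.
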(event Custom|ToggleExplode
  (if (Variables|Default|GetExplodeToggle)
    (bind _asbp_exploded_vitral_principal (Utilities|Casting|CastToBP_Exploded_VitralPrincipalClass (Variables|Default|GetVitral_to_Explode%20))
      (:then
        (bind _returnvalue (Game|SpawnActorfromClass _asbp_exploded_vitral_principal (Transformation|GetWorldTransform (Variables|Default|GetDefaultSceneRoot1)) "Undefined" "MultiplyWithRoot" 0 0))
        (Rendering|Material|SetMaterial (Variables|/Script/GeometryCollectionEngine.GeometryCollectionActor|GetGeometryCollectionComponent _returnvalue) 0 0)
        (Actor|DestroyActor))
      (:CastFailed
        (Development|PrintString "Cast Failed" true true "(R=1.000000,G=0.000000,B=0.157705,A=1.000000)")))
    (else
      (Development|PrintString "Not time to explode yet" true true "(R=1.000000,G=0.090404,B=0.850074,A=1.000000)"))))

(event EventBeginPlay)

(event Collision|EventActorBeginOverlap
  (params (OtherActor :type Actor%20Object%20Reference)))

(event EventTick
  (params (DeltaSeconds :type Float%20%28single-precision%29)))

(fn ConstructionScript)