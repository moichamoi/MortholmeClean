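; BP_Exploded_Vitral is a breakable stained-glass window that shatters when play begins.
; BeginPlay plays a 3D boom sound, prints "BOOM", applies an upward impulse to the Geometry Collection and sweeps a Destroyer component to the Destination.
; After that half-second move, the Destroyer jumps to its initial transform with height scaled tenfold.
; A separate ToggleGtavity event only enables gravity on the Geometry Collection.
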(event Custom|ToggleGtavity
  (Physics|SetEnableGravity (Variables|Default|GetGeometryCollectionComponent) true))

(event EventBeginPlay
  (bind _destination (Variables|Default|GetDestination))
  (bind _destroyer (Variables|Default|GetDestroyer))
  (bind _returnvalue (Transformation|GetRelativeTransform _destination))
  (bind _returnvalue_2 (Transformation|GetRelativeTransform _destroyer))
  ;[0.15 0.15 0.15 0.5] Audio
  (Audio|PlaySoundatLocation "/Game/Audio/MS_VitralBoom3D.MS_VitralBoom3D" (.location (Transformation|GetRelativeTransform (Variables|Default|GetDestination))) "0, 0, 0" 1.0 1.0 0.0 "/Game/SA_VitralBoom.SA_VitralBoom" 0 0 0)
  (Development|PrintString "BOOM")
  (Physics|AddImpulse (Variables|Default|GetGeometryCollectionComponent) "0.000000,0.000000,100.000000" "None" false)
  (bind _output_get (Variables|Default|SetDestroyerStartPos (Math|Transform|MakeTransform (Math|Vector|MakeVector (.x (.location _returnvalue_2)) (.y (.location _returnvalue_2)) (* (.z (.location _returnvalue_2)) 1e+01)) (.rotation _returnvalue_2) (.scale _returnvalue_2))))
  (Components|MoveComponentTo _destroyer (Math|Vector|MakeVector (.x (.location _returnvalue)) (.y (.location _returnvalue)) (.z (.location _returnvalue))) (.rotation (Transformation|GetRelativeTransform _destroyer)) false false 0.5 true)
  (Transformation|SetRelativeTransform _destroyer _output_get false false))

(fn ConstructionScript)