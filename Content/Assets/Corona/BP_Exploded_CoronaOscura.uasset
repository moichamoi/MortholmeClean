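; BP_Exploded_CoronaOscura is a Geometry Collection actor for the Corona Oscura asset that can be exploded once.
; ToggleExplode enables gravity, adds an upward impulse, sweeps the Destroyer component to a default relative transform, then disables gravity after a short delay and sets the Exploded flag.
; A separate event only enables gravity despite its toggle name.
; Logic to save and restore the Destroyer's start transform is unconnected.
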(event Custom|ToggleGtavity
  (Physics|SetEnableGravity (Variables|Default|GetGeometryCollectionComponent) true))

(event Custom|ToggleExplode
  (bind _geometrycollectioncomponent (Variables|Default|GetGeometryCollectionComponent))
  (if (!= (Variables|Default|GetExploded) true)
    (Physics|SetEnableGravity _geometrycollectioncomponent true)
    (Development|PrintString "BOOM")
    (Physics|AddImpulse _geometrycollectioncomponent "0.000000,0.000000,100.000000" "None" false)
    (Transformation|SetRelativeTransform (Variables|Default|GetDestroyer) (Math|Transform|MakeTransform "0, 0, 0" "0, 0, 0" "1.000000,1.000000,1.000000") true false)
    (Utilities|FlowControl|Delay 0.2)
    (Physics|SetEnableGravity _geometrycollectioncomponent false)
    (Variables|Default|SetExploded true)))

(event EventBeginPlay)

(fn ConstructionScript)