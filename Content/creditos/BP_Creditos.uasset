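; BP_Creditos is an actor, apparently the credits display, that follows the player's camera.
; Each Tick calls RotateMainMenu, which passes the root component and camera manager transforms through VInterpTo and RInterpTo.
; The actor takes the resulting location but only the yaw of the rotation, so it stays upright when the camera pitches or rolls.
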(event EventBeginPlay)

(event Collision|EventActorBeginOverlap
  (params (OtherActor :type Actor%20Object%20Reference)))

(event EventTick
  (params (DeltaSeconds :type Float%20%28single-precision%29))
  (CallFunction|RotateMainMenu DeltaSeconds))

(fn ConstructionScript)

(fn RotateMainMenu
  (params (DeltaTime :type Float%20%28double-precision%29))
  (bind _returnvalue (Game|GetPlayerCameraManager 0))
  (bind _defaultsceneroot (Variables|Default|GetDefaultSceneRoot))
  (bind _rootcomponent (Variables|/Script/Engine.Actor|GetRootComponent _returnvalue))
  (Transformation|SetActorTransform (Math|Transform|MakeTransform (Math|Interpolation|VInterpTo (Transformation|GetWorldLocation _defaultsceneroot) (Transformation|GetWorldLocation _rootcomponent) DeltaTime 0.0) (Math|Rotator|MakeRotator 0.0 0.0 (.yaw (Math|Interpolation|RInterpTo (Transformation|GetWorldRotation _defaultsceneroot) (Transformation|GetWorldRotation _rootcomponent) DeltaTime 0.0))) "1.000000,1.000000,1.000000")))