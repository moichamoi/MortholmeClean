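; Actor component that disintegrates its owner's mesh as soon as play begins, then disables the owner's collision.
; BeginPlay finds the mesh by class, creates two dynamic instances of its first material, and attaches a Niagara disintegration system using the particle-flagged instance.
; Tick drives DissolveAlpha on both instances from a runtime float curve over the dissolve duration, remapping the value for the mesh only.
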(event EventBeginPlay
  ;[1 1 1] Set Source Component
  (bind _asmesh_component (Utilities|Casting|CastToMeshComponent (Actor|GetComponentbyClass (Components|GetOwner) (Variables|Default|GetComponentClass))))
  (Variables|Default|SetCurrentMeshComponent _asmesh_component)
  (Variables|Default|SetCurrentMaterial (Rendering|Material|GetMaterial _asmesh_component 0))
  (Utilities|FlowControl|Sequence
    (:then_0
      ;[1 1 1] Set Dynamic Material For Mesh
      (bind _returnvalue (Rendering|Material|CreateDynamicMaterialInstance (Variables|Default|GetCurrentMaterial) "None" "None" :!class /Script/Engine.KismetMaterialLibrary))
      (bind _output_get (Variables|Default|SetComponentMaterial_Dynamic _returnvalue))
      (Rendering|Material|SetScalarParameterValue _output_get "DissolveAlpha" 0.0 :!class /Script/Engine.MaterialInstanceDynamic)
      (Rendering|Material|SetMaterial (Variables|Default|GetCurrentMeshComponent) 0 (Variables|Default|GetComponentMaterial_Dynamic)))
    (:then_1
      ;[1 1 1] Set Dynamic Material For Particle
      (bind _returnvalue_2 (Rendering|Material|CreateDynamicMaterialInstance (Variables|Default|GetCurrentMaterial) "None" "None" :!class /Script/Engine.KismetMaterialLibrary))
      (bind _output_get_2 (Variables|Default|SetParticleMaterial_Dynamic _returnvalue_2))
      (Rendering|Material|SetScalarParameterValue _output_get_2 "IsParticle" 1.0 :!class /Script/Engine.MaterialInstanceDynamic)
      (Rendering|Material|SetScalarParameterValue (Variables|Default|GetParticleMaterial_Dynamic) "DissolveAlpha" 0.0 :!class /Script/Engine.MaterialInstanceDynamic))
    (:then_2
      ;[1 1 1] Spawn Particles
      (bind _returnvalue_3 (Niagara|SpawnSystemAttached "/Game/NiagaraFX/NS_StaticDisintegration.NS_StaticDisintegration" (Variables|Default|GetCurrentMeshComponent) "None" "0, 0, 0" "0, 0, 0" "KeepRelativeOffset" false))
      (Class|NiagaraComponent|SetVariableMaterial _returnvalue_3 "Material" (Variables|Default|GetParticleMaterial_Dynamic)))
    (:then_3
      (Variables|Default|SetBeginDissolve true))))

(event EventTick
  (params (DeltaSeconds :type Float%20%28single-precision%29))
  (if (Variables|Default|GetBeginDissolve)
    (if (< (Variables|Default|GetCurrentDuration) (Variables|Default|GetDissolveDuration))
      (bind _output_get (Variables|Default|SetCurrentDuration (+ (Variables|Default|GetCurrentDuration) DeltaSeconds)))
      (Rendering|Material|SetScalarParameterValue (Variables|Default|GetComponentMaterial_Dynamic) "DissolveAlpha" (Math|Float|MapRangeClamped (Class|KismetMathLibrary|GetRuntimeFloatCurveValue (Variables|Default|GetDissolveCurve) _output_get 0.0) 0.0 1.0 -0.5 1.0) :!class /Script/Engine.MaterialInstanceDynamic)
      (Rendering|Material|SetScalarParameterValue (Variables|Default|GetParticleMaterial_Dynamic) "DissolveAlpha" (Class|KismetMathLibrary|GetRuntimeFloatCurveValue (Variables|Default|GetDissolveCurve) _output_get 0.0) :!class /Script/Engine.MaterialInstanceDynamic)
      (else
        (Variables|Default|SetBeginDissolve false)
        (Variables|Default|SetCurrentDuration 0.0)
        (Collision|SetActorEnableCollision (Components|GetOwner) false)))))